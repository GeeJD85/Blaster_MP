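; BP_BlasterCharacter is a character Blueprint that shows the player's name on an overhead widget.
; BeginPlay casts the OverheadWidget component's user widget to WBP_OverheadWidget and caches it as DisplayText.
; Tick polls until PlayerState is valid, then sets IsNameSet and passes the character to the widget's SetPlayerName, so the name is set only once.
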(event `self.ReceiveBeginPlay`
  (`self.CreateOverheadWidget`))

(event `self.ReceiveTick`
  (params (DeltaSeconds :type "Float (single-precision)"))
  (`self.SetPlayerNameText` (`self.IsNameSet`)))

(fn `CreateOverheadWidget`
  (bind _aswbp_overhead_widget (cast `/Game/Blueprints/HUD/WBP_OverheadWidget` (`WidgetComponent.GetUserWidgetObject` (`self.OverheadWidget`))))
  (set `self.DisplayText` _aswbp_overhead_widget))

(fn `SetPlayerNameText`
  (params (Condition :type Boolean))
  (if (not Condition)
    (`/Engine/EditorBlueprintResources/StandardMacros.IsValid` (`self.PlayerState`)
      (:`Is Valid`
        (set `self.IsNameSet` true)
        (`OverheadWidget.SetPlayerName` (`self.DisplayText`) self)))))

(fn `UserConstructionScript`)