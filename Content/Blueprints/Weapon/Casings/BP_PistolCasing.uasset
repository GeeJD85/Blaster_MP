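; Pistol casing actor whose emissive glow fades over time, as if cooling down.
; On BeginPlay it creates a dynamic material on the casing mesh, reads its starting EmissivePower and derives a per-tick decrement from CoolTime and CoolRate.
; A looping timer, with a short interval randomized per casing, subtracts that decrement and updates the material, with no clamp or stop.
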(event `self.ReceiveBeginPlay`
  (`KismetSystemLibrary.K2_SetTimerDelegate` (delegate `CoolDownEvent`) (`KismetMathLibrary.RandomFloatInRange` 0.02 0.06) true)
  (bind _emissivepower (`self.CreateDynamicMaterialInstance`))
  (`self.SetEmissiveDelta` _emissivepower))

(event `CoolDownEvent`
  (`self.CoolDown`))

(fn `CoolDown`
  (set `self.EmissivePower` (- (`self.EmissivePower`) (`self.EmissivePowerDelta`)))
  (`MaterialInstanceDynamic.SetScalarParameterValue` (`self.DynamicMaterialInstance`) "EmissivePower" (`self.EmissivePower`)))

(fn `CreateDynamicMaterialInstance`
  (returns (EmissivePower :type "Float (double-precision)"))
  (bind _returnvalue (`PrimitiveComponent.CreateDynamicMaterialInstance` (`self.CasingMesh`) 0 null "None"))
  (bind _output_get (set `self.DynamicMaterialInstance` _returnvalue))
  (bind _returnvalue_2 (`MaterialInstanceDynamic.K2_GetScalarParameterValue` _output_get "EmissivePower"))
  (return _returnvalue_2))

(fn `SetEmissiveDelta`
  (params (EmissivePower :type "Float (single-precision)"))
  (bind _output_get (set `self.EmissivePower` EmissivePower))
  (set `self.EmissivePowerDelta` (* (/ _output_get (`self.CoolTime`)) (`self.CoolRate`))))

(fn `UserConstructionScript`)